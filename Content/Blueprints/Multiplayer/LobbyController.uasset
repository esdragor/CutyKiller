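; Lobby controller that shows the lobby UI and handles character choice in multiplayer.
; On BeginPlay it branches on authority, creating a LobbyHostScreen on authority and a LobbyJoinScreen on remote.
; Player list updates are stored, and only the authority side forwards them to the host screen.
; ChangeCharacter replaces and possesses the pawn at its current transform; it and SetCharacterClass save the chosen class to OnlineGameInstance.
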(event `self.ReceiveBeginPlay`
  (`self.CreateMenus`))

(event `self.ReceiveTick`
  (params (DeltaSeconds :type "Float (single-precision)")))

(event `CreateMenus`
  (`/Engine/EditorBlueprintResources/ActorMacros.Switch Has Authority`
    (:`Authority`
      (bind _returnvalue (`|CreateWidget` "/Game/Widget/LobbyHostScreen.LobbyHostScreen_C"))
      (bind _output_get (set `self.LobbyWidget` _returnvalue))
      (`UserWidget.AddToViewport` _output_get 0))
    (:`Remote`
      (bind _returnvalue_2 (`|CreateWidget` "/Game/Widget/LobbyJoinScreen.LobbyJoinScreen_C"))
      (bind _output_get_2 (set `self.LobbyWidget` _returnvalue_2))
      (`UserWidget.AddToViewport` _output_get_2 0))))

(event `UpdatePlayerList`
  (params (PlayersInfo :type "Array of /Game/Blueprints/Multiplayer/PlayerDataStructure Structure"))
  (set `self.ConnectedPlayersInfo` PlayersInfo)
  (`/Engine/EditorBlueprintResources/ActorMacros.Switch Has Authority`
    (:`Authority`
      (bind _aslobby_host_screen (cast `/Game/Widget/LobbyHostScreen` (`self.LobbyWidget`)))
      (`/Game/Widget/LobbyHostScreen.UpdatePlayerList` _aslobby_host_screen (`self.ConnectedPlayersInfo`)))))

(event `ChangeCharacter`
  (params (`New Character` :type "/Game/Blueprints/TESTBase Class Reference"))
  (bind _returnvalue (`self.K2_GetPawn`))
  (set `self.SpawnTransform` (`self.GetTransform` _returnvalue))
  (`self.K2_DestroyActor` _returnvalue)
  (bind _returnvalue_2 (`|SpawnActorFromClass` `New Character` (`self.SpawnTransform`) "Undefined" "OverrideRootScale" null null))
  (`self.Possess` _returnvalue_2)
  (bind _asonline_game_instance (cast `/Game/Blueprints/Multiplayer/OnlineGameInstance` (`GameplayStatics.GetGameInstance`)))
  (set `/Game/Blueprints/Multiplayer/OnlineGameInstance.ChoosenClass` `New Character` _asonline_game_instance))

(event `SetCharacterClass`
  (params (ChosenClass :type "/Game/Blueprints/TESTBase Class Reference"))
  (bind _asonline_game_instance (cast `/Game/Blueprints/Multiplayer/OnlineGameInstance` (`GameplayStatics.GetGameInstance`)))
  (set `/Game/Blueprints/Multiplayer/OnlineGameInstance.ChoosenClass` ChosenClass _asonline_game_instance))

(fn `UserConstructionScript`)