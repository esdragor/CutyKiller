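; LobbyGameMode is the multiplayer lobby game mode that tracks joining players and shares the player list with them.
; On PostLogin it casts the new player to LobbyController, then stores the controller and its PlayerInfo in two arrays.
; After a short delay it calls UpdatePlayerList on every stored controller with the full info array.
; It handles logins only, with no removal of departing players.
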(event `self.K2_PostLogin`
  (params (NewPlayer :type "PlayerController Object Reference"))
  (bind _aslobby_controller (cast `/Game/Blueprints/Multiplayer/LobbyController` NewPlayer))
  (`KismetArrayLibrary.Array_Add` (`self.ConnectedPlayers`) _aslobby_controller)
  (`KismetArrayLibrary.Array_Add` (`self.ConnectedPlayersInfo`) (`/Game/Blueprints/Multiplayer/LobbyController.PlayerInfo` _aslobby_controller))
  (`KismetSystemLibrary.Delay` 0.2)
  (for _array_element (`self.ConnectedPlayers`)
    (`/Game/Blueprints/Multiplayer/LobbyController.UpdatePlayerList` _array_element (`self.ConnectedPlayersInfo`))))

(fn `UserConstructionScript`)