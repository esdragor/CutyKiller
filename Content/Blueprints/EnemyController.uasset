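; EnemyController is the AI controller for enemies, running the BTEnemy behavior tree on BeginPlay.
; On perception updates, GetTargetloc accepts the Player or any WeaponBP in Trap status as a target.
; For traps, it also writes the controller's own actor location and a true flag to the Blackboard.
; Accepted targets are stored in the controlled Enemy pawn's ObjSaw variable.
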(event `self.ReceiveBeginPlay`
  (`self.RunBehaviorTree` "/Game/Blueprints/BTEnemy.BTEnemy"))

(event `self.AIPerception.OnTargetPerceptionUpdated`
  (params (Actor :type "Actor Object Reference") (Stimulus :type "AIStimulus Structure"))
  (bind _newparam (`self.GetTargetloc` Actor))
  (if _newparam
    (bind _asenemy (cast `/Game/Blueprints/Enemy` (`self.K2_GetPawn`)))
    (set `/Game/Blueprints/Enemy.ObjSaw` Actor _asenemy)))

(fn `GetTargetloc`
  (params (ActorSaw :type "Actor Object Reference"))
  (returns (NewParam :type Boolean))
  (locals (NewLocalVar_0 :type Name :default "MoveDestination") (NewLocalVar_1 :type Name :default "SeeSomebody"))
  (cast `/Game/Blueprints/Player` ActorSaw
    (:`then`
      _)
    (:`CastFailed`
      (bind _asweapon_bp (cast `/Game/Blueprints/WeaponBP` ActorSaw)
        (:`then`
          (if (`|EnumEquality` (`Weapon.status` _asweapon_bp) "Trap")
            (`BlackboardComponent.SetValueAsVector` (`AIBlueprintHelperLibrary.GetBlackboard` null) (`local.NewLocalVar_0`) (`self.K2_GetActorLocation`))
            (`BlackboardComponent.SetValueAsBool` (`AIBlueprintHelperLibrary.GetBlackboard` null) (`local.NewLocalVar_1`) true)
            (else
              (return false))))
        (:`CastFailed`
          (return false)))))
  (return true))

(fn `UserConstructionScript`)