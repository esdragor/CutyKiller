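; Base or standalone weapon actor that acts as a world pickup, spinning around its yaw axis while not equipped.
; Overlapping a Player stores the weapon as that player's TMPWeapon and shows the equipped-weapon UI through SceneManager; ending overlap clears both.
; EquippingWeapon only hides that widget, and TurnToSnap and IsAttacking are empty stubs.
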(event `self.ReceiveTick`
  (params (DeltaSeconds :type "Float (single-precision)"))
  (if (not (`self.Equipped`))
    (`self.TurnOnMap` DeltaSeconds)))

(event `self.ReceiveActorBeginOverlap`
  (params (OtherActor :type "Actor Object Reference"))
  (bind _asplayer (cast `/Game/Blueprints/Player` OtherActor))
  (set `/Game/Blueprints/Player.TMP_Weapon` self _asplayer)
  (`/Game/Blueprints/SceneManager.Show Equipped Weapon` (`self.SceneManager`)))

(event `self.ReceiveActorEndOverlap`
  (params (OtherActor :type "Actor Object Reference"))
  (bind _asplayer (cast `/Game/Blueprints/Player` OtherActor))
  (set `/Game/Blueprints/Player.TMP_Weapon` null _asplayer)
  (`/Game/Blueprints/SceneManager.Hide Equipped Widget` (`self.SceneManager`)))

(fn `Equipping weapon`
  (`/Game/Blueprints/SceneManager.Hide Equipped Widget` (`self.SceneManager`)))

(fn `IsAttacking`)

(fn `TurnOnMap`
  (params (speed :type "Float (double-precision)"))
  (bind (_returnvalue_roll _returnvalue_pitch _returnvalue_yaw) (`KismetMathLibrary.BreakRotator` (`self.K2_GetActorRotation`)))
  (`self.K2_SetActorRotation` (`KismetMathLibrary.MakeRotator` _returnvalue_roll _returnvalue_pitch (+ _returnvalue_yaw (* speed 60.0)))))

(fn `TurnToSnap`)

(fn `UserConstructionScript`)