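; AI controller for enemies that runs the BTEnemy behavior tree and filters what AI perception detects.
; Players and triggered explosion-trap weapons pass the filter and are stored on the Enemy pawn as the seen object.
; For traps, it also writes its own actor location, not the trap's, and a flag to the blackboard.
; Every tick, it copies the pawn's hit and death states into blackboard bools.
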(event `self.ReceiveBeginPlay`
  (`self.RunBehaviorTree` "/Game/Blueprints/AI/BTEnemy.BTEnemy")
  (bind _asenemy (cast `/Game/Blueprints/AI/Enemy` (`self.K2_GetPawn`)))
  (set `self.charac` _asenemy))

(event `self.AIPerception.OnTargetPerceptionUpdated`
  (params (Actor :type "Actor Object Reference") (Stimulus :type "AIStimulus Structure"))
  (bind _newparam (`self.CheckTargetParam` Actor))
  (if _newparam
    (bind _asenemy (cast `/Game/Blueprints/AI/Enemy` (`self.K2_GetPawn`)))
    (set `/Game/Blueprints/AI/Enemy.ObjSaw` Actor _asenemy)))

(event `self.ReceiveTick`
  (params (DeltaSeconds :type "Float (single-precision)"))
  (`BlackboardComponent.SetValueAsBool` (`AIBlueprintHelperLibrary.GetBlackboard` null) (`self.Key Name`) (`CutyKillerCharacter.Hit` (`self.charac`)))
  (`BlackboardComponent.SetValueAsBool` (`AIBlueprintHelperLibrary.GetBlackboard` null) (`self.Key Name_0`) (`CutyKillerCharacter.isDead` (`self.charac`))))

(fn `CheckTargetParam`
  (params (ActorSaw :type "Actor Object Reference"))
  (returns (NewParam :type Boolean))
  (locals (NewLocalVar_0 :type Name :default "MoveDestination") (NewLocalVar_1 :type Name :default "SeeSomebody"))
  (cast `/Game/Blueprints/Player` ActorSaw
    (:`then`
      _)
    (:`CastFailed`
      (bind _asweapon_bp (cast `/Game/Blueprints/WeaponBP` ActorSaw)
        (:`then`
          (if (and (`|EnumEquality` (`Weapon.status` _asweapon_bp) "TrapExplosion") (== (`Weapon.TrapEnclenched` _asweapon_bp) true))
            (`BlackboardComponent.SetValueAsVector` (`AIBlueprintHelperLibrary.GetBlackboard` null) (`local.NewLocalVar_0`) (`self.K2_GetActorLocation`))
            (`BlackboardComponent.SetValueAsBool` (`AIBlueprintHelperLibrary.GetBlackboard` null) (`local.NewLocalVar_1`) true)
            (else
              (return false))))
        (:`CastFailed`
          (return false)))))
  (return true))

(fn `UserConstructionScript`)