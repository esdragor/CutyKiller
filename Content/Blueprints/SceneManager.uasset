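; SceneManager is a scene-level manager that owns the equip widget and links itself to the weapons in the scene.
; On BeginPlay it writes its own reference into each entry of WeaponsOnScene, then creates the widget and adds it to the viewport hidden.
; Two functions, Show Equipped Weapon and Hide Equipped Widget, toggle that widget's visibility.
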(event `self.ReceiveBeginPlay`
  (for _array_element (`self.WeaponsOnScene`)
    (set `/Game/Blueprints/WeaponBP.SceneManager` self _array_element))
  (bind _returnvalue (`|CreateWidget` "/Game/Widget/EquipWidget.EquipWidget_C"))
  (bind _output_get (set `self.EquipWidget` _returnvalue))
  (`UserWidget.AddToViewport` _output_get 0)
  (`Widget.SetVisibility` (`self.EquipWidget`) "Hidden"))

(fn `Hide Equipped Widget`
  (`Widget.SetVisibility` (`self.EquipWidget`) "Hidden"))

(fn `Show Equipped Weapon`
  (`Widget.SetVisibility` (`self.EquipWidget`) "Visible"))

(fn `UserConstructionScript`)