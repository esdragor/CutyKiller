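; Player Blueprint that lets the player equip a pending weapon with the E key.
; When TMPWeapon is set, it becomes EquippedWeapon, the player's rotation resets to zero, and the weapon is flagged as equipped.
; The weapon's root attaches to the mesh's ArmSocket and its TurnToSnap function runs, then TMPWeapon is cleared.
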(event `Key|E`
  (params (Key :type "Key Structure"))
  (:`Pressed`
    (if (!= (`self.TMP_Weapon`) null)
      (bind _output_get (set `self.Equipped_weapon` (`self.TMP_Weapon`)))
      (`self.K2_SetActorRotation` (struct))
      (set `/Game/Blueprints/WeaponBP.Equipped` true _output_get)
      (`SceneComponent.K2_AttachToComponent` (`Actor.RootComponent` _output_get) (`self.Mesh`) "ArmSocket" "SnapToTarget" "SnapToTarget" "KeepRelative" true)
      (`/Game/Blueprints/WeaponBP.TurnToSnap` (`self.Equipped_weapon`))
      (set `self.TMP_Weapon` null))))

(fn `UserConstructionScript`)