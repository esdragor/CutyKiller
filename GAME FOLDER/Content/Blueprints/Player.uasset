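; Player Blueprint for a game with roles, handling weapon pickup, dropping, trap placement and equip prompts.
; BP-prefixed events attach the equipped item to the arm socket, toggle SceneManager's equip widget and clear the attack flag after a delay.
; Drop and trap functions detach the item and place it via a downward trace ahead of the player, with persistent debug drawing.
; Other events assign roles, retry until the role widget exists, and set GameStateMulti's sun speed.
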(event `self.ReceiveBeginPlay`
  (bind _returnvalue (`GameplayStatics.GetActorOfClass` "/Game/Blueprints/SceneManager.SceneManager_C"))
  (set `self.SceneManager` _returnvalue))

(event `self.OverlapBox.OnComponentBeginOverlap`
  (params (OverlappedComponent :type "PrimitiveComponent Object Reference") (OtherActor :type "Actor Object Reference") (OtherComp :type "PrimitiveComponent Object Reference") (OtherBodyIndex :type Integer) (bFromSweep :type Boolean) (SweepResult :type "HitResult Structure (by ref)")))

(event `self.OverlapBox.OnComponentEndOverlap`
  (params (OverlappedComponent :type "PrimitiveComponent Object Reference") (OtherActor :type "Actor Object Reference") (OtherComp :type "PrimitiveComponent Object Reference") (OtherBodyIndex :type Integer)))

(event `self.BPShowWidgetEquip`
  (params (showed :type Boolean))
  (bind _scenemanager (`self.SceneManager`))
  (if (`KismetSystemLibrary.IsValid` (`self.SceneManager`))
    (if showed
      (`/Game/Blueprints/SceneManager.Show Equipped Weapon` _scenemanager)
      (else
        (`/Game/Blueprints/SceneManager.Hide Equipped Widget` _scenemanager)))))

(event `self.BPInteract`
  (`SceneComponent.K2_AttachToComponent` (`Actor.RootComponent` (`self.WeaponEquipped`)) (`self.Mesh`) "ArmSocket" "SnapToTarget" "SnapToTarget" "KeepRelative" true)
  (`Weapon.BPSnap` (`self.WeaponEquipped`))
  (`/Game/Blueprints/SceneManager.Hide Equipped Widget` (`self.SceneManager`)))

(event `self.BPDropItem`
  (`self.DropItem`))

(event `self.BPSetTrap`
  (`self.SetTrap`))

(event `self.BPAttacking`
  (`KismetSystemLibrary.Delay` 0.2)
  (set `self.Attacking` false))

(event `self.BPPrintRolesOnScreen`
  (bind _returnvalue (`self.GetRole`))
  (bind _foundwidgets (`WidgetBlueprintLibrary.GetAllWidgetsOfClass` "/Game/Widget/ShowRolesWidget.ShowRolesWidget_C" :!label _label))
  (if (> (`KismetArrayLibrary.Array_Length` _foundwidgets) 0)
    (`/Game/Widget/ShowRolesWidget.PrintRole` (`|GetArrayItem` _foundwidgets) (break `InfoRole` _returnvalue) (`.color` (break `InfoRole` _returnvalue)))
    (else
      (`KismetSystemLibrary.Delay` 0.2)
      (goto _label))))

(event `AssignRoleOnClient`
  (params (Role :type "RolesOfPlayer Enum" :default "RoleNotAssigned"))
  (`self.AssignRole` Role))

(event `ModifySunSpeed`
  (params (Speed :type "Float (double-precision)"))
  (bind _asgame_state_multi (cast `/Game/Blueprints/Multiplayer/GameStateMulti` (`GameplayStatics.GetGameState`)))
  (set `/Game/Blueprints/Multiplayer/GameStateMulti.Speed` Speed _asgame_state_multi))

(fn `DropItem`
  (bind _weaponequipped (`self.WeaponEquipped`))
  (bind _returnvalue (+ (+ (`self.K2_GetActorLocation`) (* (`self.GetActorForwardVector`) (100.0 100.0 0.0))) (0.0 0.0 10.0)))
  (if (!= (`self.WeaponEquipped`) null)
    (bind _outhits (`KismetSystemLibrary.LineTraceMulti` :`Start` _returnvalue :`End` (+ _returnvalue (0.0 0.0 -200.0)) :`TraceChannel` "TraceTypeQuery1" :`DrawDebugType` "Persistent"))
    (`self.K2_DetachFromActor` _weaponequipped "KeepWorld" "KeepWorld" "KeepWorld")
    (bind (_output_bblockinghit _output_binitialoverlap _output_time _output_distance _output_location) (`GameplayStatics.BreakHitResult` (`|GetArrayItem` _outhits)))
    (`Weapon.BPDropWeapon` _weaponequipped _output_location)
    (set `self.WeaponEquipped` null)))

(fn `SetTrap`
  (bind _returnvalue (+ (+ (`self.K2_GetActorLocation`) (* (`self.GetActorForwardVector`) (100.0 100.0 0.0))) (0.0 0.0 10.0)))
  (bind _outhits (`KismetSystemLibrary.LineTraceMulti` :`Start` _returnvalue :`End` (+ _returnvalue (0.0 0.0 -200.0)) :`TraceChannel` "TraceTypeQuery1" :`DrawDebugType` "Persistent"))
  (`self.K2_DetachFromActor` (`self.WeaponEquipped`) "KeepWorld" "KeepWorld" "KeepWorld")
  (bind (_output_bblockinghit _output_binitialoverlap _output_time _output_distance _output_location) (`GameplayStatics.BreakHitResult` (`|GetArrayItem` _outhits)))
  (`self.K2_SetActorTransform` (`self.WeaponEquipped`) (`KismetMathLibrary.MakeTransform` _output_location) false false)
  (set `self.WeaponEquipped` null))

(fn `UserConstructionScript`)