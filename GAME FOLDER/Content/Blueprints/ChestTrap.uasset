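; ChestTrap is a trap actor that, once armed, kills an Enemy that overlaps it.
; On overlap it clears the enemy's seen-object reference, hides its mesh and spawns BPChaosTrap in its place.
; After a short delay it spawns an explosion emitter, deals lethal damage and destroys itself.
; Overridden parent functions resize the mesh, shrinking it on TurnToSnap and restoring full scale on IsAttacking or DropWeapon.
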(event `self.ReceiveBeginPlay`
  (`KismetSystemLibrary.Delay` 3.0))

(event `self.ReceiveActorBeginOverlap`
  (params (OtherActor :type "Actor Object Reference"))
  (bind (_returnvalue_x _returnvalue_y _returnvalue_z) (`KismetMathLibrary.BreakVector` (`self.K2_GetActorLocation`)))
  (if (`self.TrapEnclenched`)
    (bind _asenemy (cast `/Game/Blueprints/AI/Enemy` OtherActor))
    (set `/Game/Blueprints/AI/Enemy.ObjSaw` null _asenemy)
    (`PrimitiveComponent.SetCollisionEnabled` (`self.StaticMesh`) "NoCollision")
    (`SceneComponent.SetVisibility` (`self.StaticMesh`) false false)
    (`|SpawnActorFromClass` "/Game/Blueprints/BPChaosTrap.BPChaosTrap_C" (`KismetMathLibrary.MakeTransform` (`KismetMathLibrary.MakeVector` _returnvalue_x _returnvalue_y _returnvalue_z)) "Undefined" "OverrideRootScale" null null)
    (`KismetSystemLibrary.Delay` 0.7)
    (`self.DestroyExplosion`)
    (`CutyKillerCharacter.TakeAhit` _asenemy 9999.0 "TrapExplosion" self)
    (`self.K2_DestroyActor`)))

(fn `DestroyExplosion`
  (bind (_returnvalue_x _returnvalue_y _returnvalue_z) (`KismetMathLibrary.BreakVector` (`self.K2_GetActorLocation`)))
  (`GameplayStatics.SpawnEmitterAtLocation` "/Game/StarterContent/Particles/P_Explosion.P_Explosion" (`KismetMathLibrary.MakeVector` _returnvalue_x _returnvalue_y (+ _returnvalue_z 10.0)) (struct) (2.0 2.0 2.0)))

(fn `DropWeapon`
  (params (Location :type "Vector Structure"))
  (`parent.DropWeapon` Location)
  (`SceneComponent.SetWorldScale3D` (`self.StaticMesh`) (1.0 1.0 1.0)))

(fn `IsAttacking`
  (`parent.IsAttacking`)
  (`SceneComponent.SetWorldScale3D` (`self.StaticMesh`) (1.0 1.0 1.0)))

(fn `TurnToSnap`
  (`parent.TurnToSnap`)
  (`SceneComponent.SetWorldScale3D` (`self.StaticMesh`) (0.3 0.3 0.3)))

(fn `UserConstructionScript`)