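; SpawnerManager is a one-shot spawn point actor that gets the first player into the game as their chosen class.
; Shortly after BeginPlay, and only with authority, it casts player controller 0 to MapPlayerControllerBP and calls RequestUpdatePlayer with its own transform and that controller's chosen class.
; The actor destroys itself after a short delay following the request.
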(event `self.ReceiveBeginPlay`
  (`KismetSystemLibrary.Delay` 2.0)
  (`/Engine/EditorBlueprintResources/ActorMacros.Switch Has Authority`
    (:`Authority`
      (`self.SpawnClass`))))

(event `SpawnClass`
  (bind _asmap_player_controller_bp (cast `/Game/Blueprints/MapPlayerControllerBP` (`GameplayStatics.GetPlayerController` 0)))
  (`/Game/Blueprints/MapPlayerControllerBP.RequestUpdatePlayer` _asmap_player_controller_bp _asmap_player_controller_bp (`self.GetTransform`) (`/Game/Blueprints/MapPlayerControllerBP.Choosen Class` _asmap_player_controller_bp))
  (`KismetSystemLibrary.Delay` 1.0)
  (`self.K2_DestroyActor`))

(fn `UserConstructionScript`)