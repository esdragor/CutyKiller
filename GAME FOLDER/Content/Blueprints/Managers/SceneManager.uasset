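; SceneManager is a manager Blueprint that owns the on-screen widget for the equipped weapon.
; On BeginPlay it creates an EquipWidget, adds it to the viewport and starts it hidden.
; Separate show and hide functions toggle the widget's visibility, with only the hide path checking that the widget is valid first.
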(event `self.ReceiveBeginPlay`
  (bind _returnvalue (`|CreateWidget` "/Game/Widget/EquipWidget.EquipWidget_C"))
  (bind _output_get (set `self.EquipWidget` _returnvalue))
  (`UserWidget.AddToViewport` _output_get 0)
  (`Widget.SetVisibility` (`self.EquipWidget`) "Hidden"))

(fn `Hide Equipped Widget`
  (bind _equipwidget (`self.EquipWidget`))
  (`/Engine/EditorBlueprintResources/StandardMacros.IsValid` _equipwidget
    (:`Is Valid`
      (`Widget.SetVisibility` _equipwidget "Hidden"))))

(fn `Show Equipped Weapon`
  (`Widget.SetVisibility` (`self.EquipWidget`) "Visible"))

(fn `UserConstructionScript`)