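; QuestManager holds a quest database and configures the quest triggers that reference it.
; On BeginPlay it shuffles the database, waits briefly, then copies each quest's Delay into its trigger's activation duration, matched by quest ID.
; Helper functions look up quests by index or by a linear search on ID, so index lookups follow the shuffled order.
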(event `self.ReceiveBeginPlay`
  (`KismetArrayLibrary.Array_Shuffle` (`self.Database`))
  (`KismetSystemLibrary.Delay` 0.2)
  (`self.UpdateDelayOnTriggers`))

(fn `GetQuestWithID`
  (params (ID :type Integer))
  (returns (Output :type "Quest Structure (by ref)"))
  (locals (NewLocalVar_0 :type "Quest Structure"))
  (for _array_element (`self.Database`)
    (bind _output_get (set `local.NewLocalVar_0` _array_element))
    (if (== ID (break `Quest` _output_get))
      (return (`local.NewLocalVar_0`)))))

(fn `GetQuestWithIndex`
  (params (Index :type Integer))
  (returns (Output :type "Quest Structure (by ref)"))
  (return (`|GetArrayItem` (`self.Database`) Index)))

(fn `UpdateDelayOnTriggers`
  (for _array_element (`self.Triggers`)
    (bind _output (`self.GetQuestWithID` (`/Game/Blueprints/TriggerQuest.QuestID` _array_element)))
    (set `/Game/Blueprints/TriggerQuest.DurationToActivate` (`.Delay` (break `Quest` _output)) _array_element)))

(fn `UserConstructionScript`)