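; Sword weapon Blueprint, a child of a parent weapon class, that adjusts its mesh orientation when snapped or dropped.
; Shortly after BeginPlay it sets its Status to Sword.
; TurnToSnap and DropWeapon extend the parent's functions, each applying a fixed relative rotation to the static mesh.
; On drop, an authority switch calls ReplicatedTransToAll on authority or ReplicatedTransOnServer on remote, both sharing the same rotation step.
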(event `self.ReceiveBeginPlay`
  (`KismetSystemLibrary.Delay` 0.2)
  (set `self.status` "Sword"))

(event `ReplicatedTransOnServer`
  (`SceneComponent.K2_SetRelativeRotation` (`self.StaticMesh`) (struct :`Yaw` -90.0 :`Roll` -90.0) false false :!label _label))

(event `ReplicatedTransToAll`
  (goto _label))

(fn `DropWeapon`
  (params (Location :type "Vector Structure"))
  (`parent.DropWeapon` Location)
  (`/Engine/EditorBlueprintResources/ActorMacros.Switch Has Authority`
    (:`Authority`
      (`self.ReplicatedTransToAll`))
    (:`Remote`
      (`self.ReplicatedTransOnServer`))))

(fn `TurnToSnap`
  (`parent.TurnToSnap`)
  (`SceneComponent.K2_SetRelativeRotation` (`self.StaticMesh`) (struct :`Pitch` -20.0) false false))

(fn `UserConstructionScript`
  (`parent.UserConstructionScript`))