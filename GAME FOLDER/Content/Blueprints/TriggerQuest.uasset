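; TriggerQuest is a box trigger actor that links a world location to a quest ID and activation duration.
; When a Player enters, it shows the in-game trigger text if that quest is in MyQuests, then passes the duration, ID and itself to the Player whether or not one matched.
; On exit, if the widget is valid, it hides the text and clears the ID and actor reference.
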(event `self.Box.OnComponentBeginOverlap`
  (params (OverlappedComponent :type "PrimitiveComponent Object Reference") (OtherActor :type "Actor Object Reference") (OtherComp :type "PrimitiveComponent Object Reference") (OtherBodyIndex :type Integer) (bFromSweep :type Boolean) (SweepResult :type "HitResult Structure (by ref)"))
  (bind _asplayer (cast `/Game/Blueprints/TEST_Character/Player` OtherActor))
  (for _array_element (`CutyKillerCharacter.MyQuests` _asplayer)
    (if (== (break `Quest` _array_element) (`self.QuestID`))
      (`Widget.SetVisibility` (`/Game/Widget/InGameWidget.TextTrigger` (`/Game/Blueprints/TEST_Character/Player.WidgetInGame` _asplayer)) "Visible")
      (break)))
  (set `CutyKillerCharacter.TriggeredDuration` (`self.DurationToActivate`) _asplayer)
  (set `CutyKillerCharacter.TriggeredID` (`self.QuestID`) _asplayer)
  (set `/Game/Blueprints/TEST_Character/Player.TriggerObjQuest` self _asplayer))

(event `self.Box.OnComponentEndOverlap`
  (params (OverlappedComponent :type "PrimitiveComponent Object Reference") (OtherActor :type "Actor Object Reference") (OtherComp :type "PrimitiveComponent Object Reference") (OtherBodyIndex :type Integer))
  (bind _asplayer (cast `/Game/Blueprints/TEST_Character/Player` OtherActor))
  (bind _widgetingame (`/Game/Blueprints/TEST_Character/Player.WidgetInGame` _asplayer))
  (`/Engine/EditorBlueprintResources/StandardMacros.IsValid` _widgetingame
    (:`Is Valid`
      (`Widget.SetVisibility` (`/Game/Widget/InGameWidget.TextTrigger` _widgetingame) "Hidden")
      (set `CutyKillerCharacter.TriggeredID` -1 _asplayer)
      (set `/Game/Blueprints/TEST_Character/Player.TriggerObjQuest` null _asplayer))))

(fn `UserConstructionScript`)