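; Game mode that admits players up to a requested count and spawns each one as their chosen character class.
; PostLogin adds joiners to a player list until it reaches the "playercount" value from the options string, then makes extra players leave the session.
; Starting players restart at a found player start, where the SpawnDefaultPawnFor override spawns the class chosen on their MapPlayerController.
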(event `self.HandleStartingNewPlayer`
  (params (NewPlayer :type "PlayerController Object Reference"))
  (`self.RestartPlayerAtPlayerStart` NewPlayer (`self.K2_FindPlayerStart` NewPlayer)))

(event `self.K2_PostLogin`
  (params (NewPlayer :type "PlayerController Object Reference"))
  (if (< (`KismetArrayLibrary.Array_Length` (`self.PlayerList`)) (`KismetStringLibrary.Conv_StringToInt` (`KismetSystemLibrary.ParseParamValue` (`self.OptionsString`) "playercount")))
    (`KismetArrayLibrary.Array_Add` (`self.PlayerList`) NewPlayer)
    (else
      (bind _asmap_player_controller (cast `/Game/Blueprints/MapPlayerController` NewPlayer))
      (`/Game/Blueprints/MapPlayerController.LeaveSessionInProgress` _asmap_player_controller))))

(fn `SpawnDefaultPawnFor`
  (params (NewPlayer :type "Controller Object Reference") (StartSpot :type "Actor Object Reference"))
  (returns (ReturnValue :type "Pawn Object Reference"))
  (bind _asmap_player_controller (cast `/Game/Blueprints/MapPlayerController` NewPlayer))
  (`/Game/Blueprints/MapPlayerController.GetCharacterClass` _asmap_player_controller)
  (bind _returnvalue (`|SpawnActorFromClass` (`/Game/Blueprints/MapPlayerController.Choosen Class` _asmap_player_controller) (`self.GetTransform` StartSpot) "Undefined" "OverrideRootScale" null null))
  (return _returnvalue))

(fn `UserConstructionScript`)