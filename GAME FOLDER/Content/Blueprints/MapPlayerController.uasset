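; Player controller for a gameplay map in an online game, handling input mode, character class lookup and leaving the session.
; BeginPlay sets Game and UI input on player controller 0, and LeaveSessionInProgress opens the Menu level.
; GetCharacterClass copies the chosen class from the OnlineGameInstance into its own variable.
; Tab only prints a placeholder score message, and the local-controller check leads to no logic.
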(event `LeaveSessionInProgress`
  (`GameplayStatics.OpenLevelBySoftObjectPtr` "/Game/Level/Menu.Menu"))

(event `self.ReceiveBeginPlay`
  (`WidgetBlueprintLibrary.SetInputMode_GameAndUIEx` (`GameplayStatics.GetPlayerController` 0) null "DoNotLock" false)
  (if (`self.IsLocalPlayerController`)
    _))

(event `GetCharacterClass`
  (bind _asonline_game_instance (cast `/Game/Blueprints/Multiplayer/OnlineGameInstance` (`GameplayStatics.GetGameInstance`)))
  (set `self.Choosen Class` (`/Game/Blueprints/Multiplayer/OnlineGameInstance.ChoosenClass` _asonline_game_instance)))

(event `Key|Tab`
  (params (Key :type "Key Structure"))
  (:`Pressed`
    (`KismetSystemLibrary.PrintString` "print score")))

(fn `UserConstructionScript`)