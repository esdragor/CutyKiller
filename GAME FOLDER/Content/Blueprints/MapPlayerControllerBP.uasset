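; Player controller for an online map that handles input mode, chosen character class, the player list and leaving the session.
; BeginPlay sets Game and UI input, and GetCharacterClass copies the chosen class from OnlineGameInstance.
; Pressing Tab creates a new player list widget on the authority side only.
; LeaveSessionInProgress opens the Menu level with a "kicked" option.
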(event `LeaveSessionInProgress`
  (`GameplayStatics.OpenLevelBySoftObjectPtr` "/Game/Level/Menu.Menu" true "kicked"))

(event `self.ReceiveBeginPlay`
  (`WidgetBlueprintLibrary.SetInputMode_GameAndUIEx` (`GameplayStatics.GetPlayerController` 0) null "DoNotLock" false))

(event `GetCharacterClass`
  (bind _asonline_game_instance (cast `/Game/Blueprints/Multiplayer/OnlineGameInstance` (`GameplayStatics.GetGameInstance`)))
  (set `self.Choosen Class` (`/Game/Blueprints/Multiplayer/OnlineGameInstance.ChoosenClass` _asonline_game_instance)))

(event `Key|Tab`
  (params (Key :type "Key Structure"))
  (:`Pressed`
    (`/Engine/EditorBlueprintResources/ActorMacros.Switch Has Authority`
      (:`Authority`
        (bind _returnvalue (`|CreateWidget` "/Game/Widget/PlayerListWidget.PlayerListWidget_C"))
        (bind _output_get (set `self.PlayerListWidget` _returnvalue))
        (`UserWidget.AddToViewport` _output_get 0)))))

(fn `UserConstructionScript`)