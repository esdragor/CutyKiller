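; Base weapon actor that spins around its yaw axis each tick while unequipped, like a pickup lying on the map.
; Drop requests pass through DropWeaponOnServer to DropWeapon, which clears Equipped and repositions the actor 20 units above the given location.
; The snap event calls TurnToSnap, which is an empty stub, as is IsAttacking.
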(event `self.ReceiveTick`
  (params (DeltaSeconds :type "Float (single-precision)"))
  (if (not (`self.Equipped`))
    (`self.TurnOnMap` DeltaSeconds)))

(event `self.BPSnap`
  (`self.TurnToSnap`))

(event `self.BPDropWeapon`
  (params (Location :type "Vector Structure"))
  (`self.DropWeaponOnServer` Location))

(event `DropWeaponOnServer`
  (params (Location :type "Vector Structure"))
  (`self.DropWeapon` Location))

(fn `DropWeapon`
  (params (Location :type "Vector Structure"))
  (set `self.Equipped` false)
  (`self.K2_SetActorTransform` (`KismetMathLibrary.MakeTransform` (- Location (0.0 0.0 -20.0)))))

(fn `IsAttacking`)

(fn `TurnOnMap`
  (params (speed :type "Float (double-precision)"))
  (bind (_returnvalue_roll _returnvalue_pitch _returnvalue_yaw) (`KismetMathLibrary.BreakRotator` (`self.K2_GetActorRotation`)))
  (`self.K2_SetActorRotation` (`KismetMathLibrary.MakeRotator` _returnvalue_roll _returnvalue_pitch (+ _returnvalue_yaw (* speed 60.0)))))

(fn `TurnToSnap`)

(fn `UserConstructionScript`)