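; Multiplayer lobby player controller that manages lobby menus, character choice, ready state and kicking.
; An authority switch creates the host or join screen and routes player list updates to it.
; Character changes replace the pawn in place and save the chosen class in OnlineGameInstance.
; Possession and ready toggles update PlayerInfo and make LobbyGameMode refresh player lists, while a kick opens the Menu level with a "kicked" option.
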(event `self.ReceiveBeginPlay`
  (`self.CreateMenus`))

(event `self.ReceiveTick`
  (params (DeltaSeconds :type "Float (single-precision)")))

(event `CreateMenus`
  (`/Engine/EditorBlueprintResources/ActorMacros.Switch Has Authority`
    (:`Authority`
      (bind _returnvalue (`|CreateWidget` "/Game/Widget/LobbyHostScreen.LobbyHostScreen_C"))
      (bind _output_get (set `self.LobbyWidget` _returnvalue))
      (`UserWidget.AddToViewport` _output_get 0))
    (:`Remote`
      (bind _returnvalue_2 (`|CreateWidget` "/Game/Widget/LobbyJoinScreen.LobbyJoinScreen_C"))
      (bind _output_get_2 (set `self.LobbyWidget` _returnvalue_2))
      (`UserWidget.AddToViewport` _output_get_2 0))))

(event `UpdatePlayerList`
  (params (PlayersInfo :type "Array of /Game/Blueprints/Multiplayer/PlayerDataStructure Structure"))
  (bind _lobbywidget (`self.LobbyWidget`))
  (bind _connectedplayersinfo (`self.ConnectedPlayersInfo`))
  (set `self.ConnectedPlayersInfo` PlayersInfo)
  (`/Engine/EditorBlueprintResources/ActorMacros.Switch Has Authority`
    (:`Authority`
      (bind _aslobby_host_screen (cast `/Game/Widget/LobbyHostScreen` _lobbywidget))
      (`/Game/Widget/LobbyHostScreen.UpdatePlayerList` _aslobby_host_screen _connectedplayersinfo))
    (:`Remote`
      (bind _aslobby_join_screen (cast `/Game/Widget/LobbyJoinScreen` _lobbywidget))
      (`/Game/Widget/LobbyJoinScreen.UpdatePlayerList` _aslobby_join_screen _connectedplayersinfo))))

(event `ChangeCharacter`
  (params (`New Character` :type "/Game/Blueprints/TESTBase Class Reference"))
  (bind _returnvalue (`self.K2_GetPawn`))
  (set `self.SpawnTransform` (`self.GetTransform` _returnvalue))
  (`self.K2_DestroyActor` _returnvalue)
  (bind _returnvalue_2 (`|SpawnActorFromClass` `New Character` (`self.SpawnTransform`) "Undefined" "OverrideRootScale" null null))
  (`self.Possess` _returnvalue_2)
  (bind _asonline_game_instance (cast `/Game/Blueprints/Multiplayer/OnlineGameInstance` (`GameplayStatics.GetGameInstance`)))
  (set `/Game/Blueprints/Multiplayer/OnlineGameInstance.ChoosenClass` `New Character` _asonline_game_instance))

(event `SetCharacterClass`
  (params (ChosenClass :type "/Game/Blueprints/TESTBase Class Reference"))
  (bind _asonline_game_instance (cast `/Game/Blueprints/Multiplayer/OnlineGameInstance` (`GameplayStatics.GetGameInstance`)))
  (set `/Game/Blueprints/Multiplayer/OnlineGameInstance.ChoosenClass` ChosenClass _asonline_game_instance))

(event `SetReadyStatut`
  (bind _playerinfo (`self.PlayerInfo`))
  (setmembers `/Game/Blueprints/Multiplayer/PlayerDataStructure` :`StructRef` _playerinfo :`IsReady` (not (`.IsReady_4_ABD0609C44CACB66F6F9D08ADAE80EF0` (break `/Game/Blueprints/Multiplayer/PlayerDataStructure` _playerinfo))))
  (bind _aslobby_game_mode (cast `/Game/Blueprints/Multiplayer/LobbyGameMode` (`GameplayStatics.GetGameMode`)))
  (`/Game/Blueprints/Multiplayer/LobbyGameMode.UpdatePlayerLists` _aslobby_game_mode))

(event `self.ReceivePossess`
  (params (PossessedPawn :type "Pawn Object Reference"))
  (setmembers `/Game/Blueprints/Multiplayer/PlayerDataStructure` :`StructRef` (`self.PlayerInfo`) :`Character` PossessedPawn)
  (bind _aslobby_game_mode (cast `/Game/Blueprints/Multiplayer/LobbyGameMode` (`GameplayStatics.GetGameMode`)))
  (`/Game/Blueprints/Multiplayer/LobbyGameMode.UpdatePlayerLists` _aslobby_game_mode))

(event `KickedFromLobby`
  (`GameplayStatics.OpenLevelBySoftObjectPtr` "/Game/Level/Menu.Menu" true "kicked"))

(fn `UserConstructionScript`)