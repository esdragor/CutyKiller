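; Lobby game mode that tracks connected LobbyControllers and pushes the player list to each of them.
; On PostLogin it fills PlayerInfo with the local GameInstance's name, marking the host ready and clients not ready; client entries get appended twice.
; Logout removes the controller and calls UpdatePlayerLists, which rebuilds the list from each controller's info.
; Both login and rebuild broadcast after a short delay.
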(event `self.K2_PostLogin`
  (params (NewPlayer :type "PlayerController Object Reference"))
  (bind _aslobby_controller (cast `/Game/Blueprints/Multiplayer/LobbyController` NewPlayer))
  (`KismetArrayLibrary.Array_Add` (`self.ConnectedPlayers`) _aslobby_controller)
  (if (`Controller.IsLocalController` _aslobby_controller)
    (`self.Make Host Ready` _aslobby_controller)
    (else
      (`self.Set Name Client` _aslobby_controller)
      (`KismetArrayLibrary.Array_Add` (`self.ConnectedPlayersInfo`) (`/Game/Blueprints/Multiplayer/LobbyController.PlayerInfo` _aslobby_controller))))
  (`KismetSystemLibrary.Delay` 0.2)
  (for _array_element (`self.ConnectedPlayers`)
    (`/Game/Blueprints/Multiplayer/LobbyController.UpdatePlayerList` _array_element (`self.ConnectedPlayersInfo`))))

(event `UpdatePlayerLists`
  (`KismetArrayLibrary.Array_Clear` (`self.ConnectedPlayersInfo`))
  (for _array_element (`self.ConnectedPlayers`)
    (if (`Controller.IsLocalController` _array_element)
      (`self.Make Host Ready` _array_element)
      (else
        (`KismetArrayLibrary.Array_Add` (`self.ConnectedPlayersInfo`) (`/Game/Blueprints/Multiplayer/LobbyController.PlayerInfo` _array_element)))))
  (`KismetSystemLibrary.Delay` 0.2)
  (for _array_element_2 (`self.ConnectedPlayers`)
    (`/Game/Blueprints/Multiplayer/LobbyController.UpdatePlayerList` _array_element_2 (`self.ConnectedPlayersInfo`))))

(event `self.K2_OnLogout`
  (params (ExitingController :type "Controller Object Reference"))
  (bind _aslobby_controller (cast `/Game/Blueprints/Multiplayer/LobbyController` ExitingController))
  (`KismetArrayLibrary.Array_RemoveItem` (`self.ConnectedPlayers`) _aslobby_controller)
  (`self.UpdatePlayerLists`))

(fn `Make Host Ready`
  (params (LobbyController :type "/Game/Blueprints/Multiplayer/LobbyController Object Reference"))
  (bind _asonline_game_instance (cast `/Game/Blueprints/Multiplayer/OnlineGameInstance` (`GameplayStatics.GetGameInstance`)))
  (bind _output_get (set `/Game/Blueprints/Multiplayer/LobbyController.PlayerInfo` (make `/Game/Blueprints/Multiplayer/PlayerDataStructure` (`KismetTextLibrary.Conv_StringToText` (`KismetStringLibrary.Conv_NameToString` (`GameInstanceUtility.NameOfPlayer` _asonline_game_instance))) true) LobbyController))
  (`KismetArrayLibrary.Array_Add` (`self.ConnectedPlayersInfo`) _output_get))

(fn `Set Name Client`
  (params (LobbyController :type "/Game/Blueprints/Multiplayer/LobbyController Object Reference"))
  (bind _asonline_game_instance (cast `/Game/Blueprints/Multiplayer/OnlineGameInstance` (`GameplayStatics.GetGameInstance`)))
  (bind _output_get (set `/Game/Blueprints/Multiplayer/LobbyController.PlayerInfo` (make `/Game/Blueprints/Multiplayer/PlayerDataStructure` (`KismetTextLibrary.Conv_StringToText` (`KismetStringLibrary.Conv_NameToString` (`GameInstanceUtility.NameOfPlayer` _asonline_game_instance)))) LobbyController))
  (`KismetArrayLibrary.Array_Add` (`self.ConnectedPlayersInfo`) _output_get))

(fn `UserConstructionScript`)