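; Multiplayer game state Blueprint that shows the roles widget when play begins and sets up a day-night cycle.
; BeginPlay adds the widget to the viewport, stores the first DirectionalLight found and calls NightDayCycle.
; That event is empty, so the cycle does nothing.
; A disconnected chain holds the intended loop: pitch the light by Speed and delta time, run CheckDayNight, then repeat after a short Delay.
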(event `self.ReceiveBeginPlay`
  (bind _returnvalue (`|CreateWidget` "/Game/Widget/ShowRolesWidget.ShowRolesWidget_C"))
  (`UserWidget.AddToViewport` _returnvalue 0)
  (bind _outactors (`GameplayStatics.GetAllActorsOfClass` "/Script/Engine.DirectionalLight"))
  (set `self.Light` (`|GetArrayItem` _outactors))
  (`self.NightDayCycle`))

(event `NightDayCycle`)

(fn `UserConstructionScript`)