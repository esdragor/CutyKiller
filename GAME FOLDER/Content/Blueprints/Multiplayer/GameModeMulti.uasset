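; Multiplayer game mode for a hidden-role match of Killers versus GoodGuys, spawning each player's pawn from the GameInstance's chosen class.
; PostLogin tracks players up to the session's playercount option and makes extras leave.
; BeginPlay polls until all players join, then deals shuffled roles, starts client quests and sets day-night sun speed.
; Victory calls accumulate points, notifying every player once points reach the non-killer count.
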(event `self.HandleStartingNewPlayer`
  (params (NewPlayer :type "PlayerController Object Reference"))
  (`self.RestartPlayerAtPlayerStart` NewPlayer (`self.K2_FindPlayerStart` NewPlayer)))

(event `self.ReceiveBeginPlay`
  (`KismetSystemLibrary.Delay` 0.3)
  (`self.RestartPlayer` (`GameplayStatics.GetPlayerController` 0))
  (bind _asonline_game_instance (cast `/Game/Blueprints/Multiplayer/OnlineGameInstance` (`GameplayStatics.GetGameInstance`) :!label _label))
  (if (<= (`/Game/Blueprints/Multiplayer/OnlineGameInstance.Nb Players` _asonline_game_instance) (`KismetArrayLibrary.Array_Length` (`self.PlayerList`)))
    (`self.InitRolesOnServer`)
    (`self.StartDayNightCycle`)
    (else
      (`KismetSystemLibrary.Delay` 0.2)
      (goto _label))))

(event `self.K2_PostLogin`
  (params (NewPlayer :type "PlayerController Object Reference"))
  (if (< (`KismetArrayLibrary.Array_Length` (`self.PlayerList`)) (`KismetStringLibrary.Conv_StringToInt` (`KismetSystemLibrary.ParseParamValue` (`self.OptionsString`) "playercount")))
    (`KismetArrayLibrary.Array_Add` (`self.PlayerList`) NewPlayer)
    (else
      (bind _asmap_player_controller_bp (cast `/Game/Blueprints/MapPlayerControllerBP` NewPlayer))
      (`/Game/Blueprints/MapPlayerControllerBP.LeaveSessionInProgress` _asmap_player_controller_bp))))

(event `Respawn`
  (params (controller :type "PlayerController Object Reference") (`Spawn Transform` :type "Transform Structure") (Class :type "/Game/Blueprints/TEST_Character/Player Class Reference"))
  (`/Engine/EditorBlueprintResources/StandardMacros.IsValid` controller
    (:`Is Valid`
      (bind _returnvalue (`|SpawnActorFromClass` Class `Spawn Transform` "Undefined" "OverrideRootScale" null null))
      (`KismetSystemLibrary.Delay` 0.2)
      (`Controller.Possess` controller _returnvalue)
      (cast `/Game/Blueprints/MapPlayerControllerBP` controller))))

(event `InitRolesOnServer`
  ;[1 1 1] assignation roles
  (`KismetSystemLibrary.Delay` 0.2)
  (`self.InitRoles`)
  (for (_array_element _array_index) (`self.PlayerList`)
    (bind _asplayer (cast `/Game/Blueprints/TEST_Character/Player` (`Controller.K2_GetPawn` _array_element)))
    (`/Game/Blueprints/TEST_Character/Player.AssignRoleOnClient` _asplayer (`|GetArrayItem` (`self.AssignedRoles`) _array_index))
    (`/Game/Blueprints/TEST_Character/Player.InitQuestInClient` _asplayer 0)))

(event `StartDayNightCycle`
  (`KismetSystemLibrary.Delay` 0.2)
  (bind _asonline_game_instance (cast `/Game/Blueprints/Multiplayer/OnlineGameInstance` (`GameplayStatics.GetGameInstance`)))
  (for _array_element (`self.PlayerList`)
    (bind _asplayer (cast `/Game/Blueprints/TEST_Character/Player` (`Controller.K2_GetPawn` _array_element)))
    (`/Game/Blueprints/TEST_Character/Player.ModifySunSpeed` _asplayer (`GameInstanceUtility.SpeedCycleDayNight` _asonline_game_instance))))

(event `CheckVictoryToAll`
  (bind _result (`/Engine/EditorBlueprintResources/StandardMacros.IncrementInt` (`self.VictoryPoints`))
    (:`  `
      (bind _asonline_game_instance (cast `/Game/Blueprints/Multiplayer/OnlineGameInstance` (`GameplayStatics.GetGameInstance`)))
      (if (>= _result (- (`KismetArrayLibrary.Array_Length` (`self.PlayerList`)) (`GameInstanceUtility.NbKIllersToCreate` _asonline_game_instance)))
        (for _array_element (`self.PlayerList`)
          (bind _asplayer (cast `/Game/Blueprints/TEST_Character/Player` (`Controller.K2_GetPawn` _array_element)))
          (`/Game/Blueprints/TEST_Character/Player.VictoryOnClient` _asplayer))))))

(fn `InitRoles`
  (locals (GameState :type "Object Object Reference"))
  (bind _assignedroles (`self.AssignedRoles`))
  (if (<= (`KismetArrayLibrary.Array_Length` (`self.AssignedRoles`)) 0)
    (bind _asonline_game_instance (cast `/Game/Blueprints/Multiplayer/OnlineGameInstance` (`GameplayStatics.GetGameInstance`)))
    (bind _nbkillerstocreate (`GameInstanceUtility.NbKIllersToCreate` _asonline_game_instance))
    (if (> _nbkillerstocreate 0)
      (for _ (range 1 (+ _nbkillerstocreate 1))
        (`KismetArrayLibrary.Array_Add` (`self.AssignedRoles`) "Killer")))
    (for _ (range (+ _nbkillerstocreate 1) (+ (`/Game/Blueprints/Multiplayer/OnlineGameInstance.Nb Players` _asonline_game_instance) 1))
      (`KismetArrayLibrary.Array_Add` _assignedroles "GoodGuy"))
    (`KismetArrayLibrary.Array_Shuffle` _assignedroles)))

(fn `SpawnDefaultPawnFor`
  (params (NewPlayer :type "Controller Object Reference") (StartSpot :type "Actor Object Reference"))
  (returns (ReturnValue :type "Pawn Object Reference"))
  (bind _asmap_player_controller_bp (cast `/Game/Blueprints/MapPlayerControllerBP` NewPlayer))
  (`/Game/Blueprints/MapPlayerControllerBP.GetCharacterClass` _asmap_player_controller_bp)
  (bind _asonline_game_instance (cast `/Game/Blueprints/Multiplayer/OnlineGameInstance` (`GameplayStatics.GetGameInstance`)))
  (bind _returnvalue (`|SpawnActorFromClass` (`/Game/Blueprints/Multiplayer/OnlineGameInstance.ChoosenClass` _asonline_game_instance) (`self.GetTransform` StartSpot) "Undefined" "OverrideRootScale" null null))
  (return _returnvalue))

(fn `UserConstructionScript`)