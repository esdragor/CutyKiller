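; Dog character Blueprint (chien) whose power depends on its role.
; For the Naughty role, the power triggers dog vision on the WallHackVisionManager.
; Otherwise it finds a navigation path to the closest Player and copies the path points into a spline.
; PrintSplineMesh draws that trail with one runtime spline mesh per segment, and the meshes are destroyed after a delay.
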(event `self.BPPower`
  (bind _splinemeshes (`self.SplineMeshes`))
  (bind _returnvalue (`self.GetRoleParameters`))
  (if (`|EnumEquality` (`.typeOfRoles` (break `InfoRole` _returnvalue)) "Naughty")
    (bind _outactors (`GameplayStatics.GetAllActorsOfClass` "/Game/Blueprints/WallHackVisionManager.WallHackVisionManager_C"))
    (if (> (`KismetArrayLibrary.Array_Length` _outactors) 0)
      (`/Game/Blueprints/WallHackVisionManager.GestionDogVision` (`|GetArrayItem` _outactors)))
    (else
      (bind _outactors_2 (`GameplayStatics.GetAllActorsOfClass` "/Game/Blueprints/TEST_Character/Player.Player_C"))
      (bind _returnvalue_2 (`self.FindClosestPlayer` _outactors_2))
      (`/Engine/EditorBlueprintResources/StandardMacros.IsValid` _returnvalue_2
        (:`Is Valid`
          (bind _returnvalue_3 (`NavigationSystemV1.FindPathToLocationSynchronously` (`self.K2_GetActorLocation`) (`self.K2_GetActorLocation` _returnvalue_2) null null))
          (`SplineComponent.ClearSplinePoints` (`self.Spline`) true)
          (for _array_element (`NavigationPath.PathPoints` _returnvalue_3)
            (`SplineComponent.AddSplinePoint` (`self.Spline`) _array_element "World" true))
          (`self.PrintSplineMesh`)
          (`KismetSystemLibrary.Delay` 10.0)
          (for _array_element_2 _splinemeshes
            (`ActorComponent.K2_DestroyComponent` _array_element_2))
          (`KismetArrayLibrary.Array_Clear` _splinemeshes))))))

(fn `PrintSplineMesh`
  (bind _spline (`self.Spline`))
  (bind _splinemeshes (`self.SplineMeshes`))
  (for _array_element _splinemeshes
    (`ActorComponent.K2_DestroyComponent` _array_element))
  (`KismetArrayLibrary.Array_Clear` _splinemeshes)
  (for _index (range (`SplineComponent.GetNumberOfSplineSegments` _spline))
    (bind _returnvalue (`AddComponent|NODE_AddSplineMeshComponent-0`))
    (`SceneComponent.K2_DetachFromComponent` _returnvalue "KeepWorld" "KeepWorld" "KeepWorld" true)
    (`KismetArrayLibrary.Array_Add` (`self.SplineMeshes`) _returnvalue)
    (bind (_location _tangent) (`SplineComponent.GetLocationAndTangentAtSplinePoint` _spline _index "Local"))
    (bind (_location_2 _tangent_2) (`SplineComponent.GetLocationAndTangentAtSplinePoint` _spline (+ _index 1) "Local"))
    (`SplineMeshComponent.SetStartAndEnd` _returnvalue _location _tangent _location_2 _tangent_2 true)))

(fn `UserConstructionScript`
  (`parent.UserConstructionScript`))