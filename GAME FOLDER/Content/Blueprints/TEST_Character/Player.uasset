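; Player character Blueprint for a multiplayer hidden-role game where Good and Naughty sides win through quests or kills.
; BP-prefixed events branch on authority into paired ToAll/OnServer events for weapon pickup, drop, traps, attacks and death.
; Delay-and-retry loops wait for widgets before showing role, powers and non-Naughty quests in the HUD.
; Quest completion and kill checks go to GameModeMulti; client events show victory or defeat by role type.
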(event `CanMove`
  (set `self.cantMove` false))

(event `self.ReceiveBeginPlay`
  (bind _returnvalue (`GameplayStatics.GetActorOfClass` "/Game/Blueprints/Managers/SceneManager.SceneManager_C"))
  (set `self.SceneManager` _returnvalue))

(event `ModifySunSpeed`
  (params (Speed :type "Float (double-precision)"))
  (bind _asgame_state_multi (cast `/Game/Blueprints/Multiplayer/GameStateMulti` (`GameplayStatics.GetGameState`)))
  (set `/Game/Blueprints/Multiplayer/GameStateMulti.Speed` Speed _asgame_state_multi))

(event `self.BPShowEquippedWidget`
  (params (IsShow :type Boolean))
  (bind _scenemanager (`self.SceneManager`))
  ;[1 1 1] WeaponManager
  (if (`KismetSystemLibrary.IsValid` (`self.SceneManager`))
    (if IsShow
      (`/Game/Blueprints/Managers/SceneManager.Show Equipped Weapon` _scenemanager)
      (else
        (`/Game/Blueprints/Managers/SceneManager.Hide Equipped Widget` _scenemanager)))))

(event `self.BPPrintRolesOnScreen`
  ;[1 1 1] RoleManager
  (bind _returnvalue (`self.GetRoleParameters`))
  (bind _foundwidgets (`WidgetBlueprintLibrary.GetAllWidgetsOfClass` "/Game/Widget/ShowRolesWidget.ShowRolesWidget_C" :!label _label))
  (if (> (`KismetArrayLibrary.Array_Length` _foundwidgets) 0)
    (`/Game/Widget/ShowRolesWidget.PrintRole` (`|GetArrayItem` _foundwidgets) (break `InfoRole` _returnvalue) (`.color` (break `InfoRole` _returnvalue)))
    (`KismetSystemLibrary.Delay` 1.0)
    (`self.InitCam`)
    (`KismetSystemLibrary.Delay` 4.0)
    (bind _foundwidgets_2 (`WidgetBlueprintLibrary.GetAllWidgetsOfClass` "/Game/Widget/InGameWidget.InGameWidget_C"))
    (bind _output_get (set `self.WidgetInGame` (`|GetArrayItem` _foundwidgets_2)))
    (`/Game/Widget/InGameWidget.ShowHideInGame` _output_get "Visible")
    (`Widget.SetVisibility` (`/Game/Widget/InGameWidget.CanvasPanel_31` _output_get) "SelfHitTestInvisible")
    (`self.InitPower`)
    (else
      (`KismetSystemLibrary.Delay` 0.2)
      (goto _label))))

(event `ReplicateTakeOnServer`
  (params (Weapon :type "Weapon Object Reference") (Parent :type "SceneComponent Object Reference"))
  ;[1 1 1] WeaponManager
  (`SceneComponent.K2_AttachToComponent` (`Actor.RootComponent` Weapon) Parent "ArmSocket" "SnapToTarget" "SnapToTarget" "KeepRelative" true)
  (`Weapon.BPSnap` Weapon)
  (`/Game/Blueprints/Managers/SceneManager.Hide Equipped Widget` (`self.SceneManager`))
  (set `Weapon.Equipped` true Weapon)
  (`self.SetWeaponEquip` Weapon))

(event `AssignRoleOnClient`
  (params (Role :type "RolesOfPlayer Enum" :default "RoleNotAssigned"))
  ;[1 1 1] RoleManager
  (`self.AssignRole` Role)
  (`KismetSystemLibrary.Delay` 1.0)
  (`self.AssignAnimal`))

(event `ReplicateTakeToAll`
  (params (Weapon :type "Weapon Object Reference") (Parent :type "SceneComponent Object Reference"))
  ;[1 1 1] WeaponManager
  (`SceneComponent.K2_AttachToComponent` (`Actor.RootComponent` Weapon) Parent "ArmSocket" "SnapToTarget" "SnapToTarget" "KeepRelative" true)
  (`Weapon.BPSnap` Weapon)
  (`/Game/Blueprints/Managers/SceneManager.Hide Equipped Widget` (`self.SceneManager`))
  (set `Weapon.Equipped` true Weapon)
  (`self.SetWeaponEquip` Weapon))

(event `self.BPInteract`
  ;[1 1 1] WeaponManager
  (`/Engine/EditorBlueprintResources/ActorMacros.Switch Has Authority`
    (:`Authority`
      (`self.ReplicateTakeToAll` (`self.WeaponEquipped`) (`self.Mesh`)))
    (:`Remote`
      (`self.ReplicateTakeOnServer` (`self.WeaponEquipped`) (`self.Mesh`)))))

(event `InitQuestInClient`
  (params (nbQuest :type Integer))
  ;[1 1 1] Quest manage
  (bind _returnvalue (`self.GetRoleParameters`))
  (if (`|EnumInequality` (`.typeOfRoles` (break `InfoRole` _returnvalue)) "Naughty")
    (bind _outactors (`GameplayStatics.GetAllActorsOfClass` "/Game/Blueprints/Managers/QuestManager.QuestManager_C"))
    (for _index (range (+ nbQuest 1))
      (bind _output (`/Game/Blueprints/Managers/QuestManager.GetQuestWithIndex` (`|GetArrayItem` _outactors) _index))
      (`KismetArrayLibrary.Array_Add` (`self.MyQuests`) _output))
    (`KismetSystemLibrary.Delay` 0.2 :!label _label_2)
    (`/Engine/EditorBlueprintResources/StandardMacros.IsValid` (`self.WidgetInGame`)
      (:`Is Valid`
        (`KismetSystemLibrary.Delay` 0.2)
        (for (_array_element _array_index) (`self.MyQuests`)
          (`/Game/Widget/InGameWidget.AddQuest` (`self.WidgetInGame`) _array_element _array_index)))
      (:`Is Not Valid`
        (goto _label_2)))))

(event `ReplicateDropOnServer`
  ;[1 1 1] WeaponManager
  (`self.DropItem` :!label _label_3))

(event `self.BPDropItem`
  ;[1 1 1] WeaponManager
  (`/Engine/EditorBlueprintResources/ActorMacros.Switch Has Authority`
    (:`Authority`
      (`self.ReplicateDropToAll`))
    (:`Remote`
      (`self.ReplicateDropOnServer`))))

(event `ReplicateDropToAll`
  ;[1 1 1] WeaponManager
  (goto _label_3))

(event `self.BPSetTrap`
  ;[1 1 1] WeaponManager
  (`/Engine/EditorBlueprintResources/ActorMacros.Switch Has Authority`
    (:`Authority`
      (`self.ReplicatedSetTrapToAll`))
    (:`Remote`
      (`self.ReplicatedSetTrapOnServer`))))

(event `ReplicatedSetTrapToAll`
  ;[1 1 1] WeaponManager
  (`self.SetTrap` :!label _label_4))

(event `ReplicatedSetTrapOnServer`
  ;[1 1 1] WeaponManager
  (goto _label_4))

(event `self.SwitchDayNight`
  (params (IsNight :type Boolean))
  (bind _spotlight (`self.SpotLight`))
  (if IsNight
    (`SceneComponent.SetVisibility` _spotlight true false)
    (else
      (`SceneComponent.SetVisibility` _spotlight false false))))

(event `ReplicatedAttackToAll`
  (params (weapon :type "Weapon Object Reference"))
  ;[1 1 1] WeaponManager
  (`self.SetWeaponEquip` weapon)
  (set `self.Attacking` true :!label _label_5)
  (`KismetSystemLibrary.Delay` 0.2)
  (set `self.Attacking` false))

(event `self.BPAttacking`
  (bind _weaponequipped (`self.WeaponEquipped`))
  ;[1 1 1] WeaponManager
  (`/Engine/EditorBlueprintResources/ActorMacros.Switch Has Authority`
    (:`Authority`
      (`self.ReplicatedAttackToAll` _weaponequipped))
    (:`Remote`
      (`self.ReplicateAttackValueOnServer` _weaponequipped))))

(event `ReplicateAttackValueOnServer`
  (params (Weapon :type "Weapon Object Reference"))
  ;[1 1 1] WeaponManager
  (`self.SetWeaponEquip` Weapon)
  (goto _label_5))

(event `self.BPUpdateQuest`
  (bind _triggerobjquest (`self.TriggerObjQuest`))
  (bind _myquests (`self.MyQuests`))
  (`/Engine/EditorBlueprintResources/StandardMacros.IsValid` _triggerobjquest
    (:`Is Valid`
      (`self.K2_DestroyActor` _triggerobjquest))
    (:`Is Not Valid`
      _))
  (`/Game/Widget/InGameWidget.ClearQuestBox` (`self.WidgetInGame`))
  (for (_array_element _array_index) _myquests
    (`/Game/Widget/InGameWidget.AddQuest` (`self.WidgetInGame`) _array_element _array_index))
  (if (== (`KismetArrayLibrary.Array_Length` _myquests) 0)
    (`/Engine/EditorBlueprintResources/ActorMacros.Switch Has Authority`
      (:`Authority`
        (`/Engine/EditorBlueprintResources/StandardMacros.FlipFlop`
          (:`A`
            _)))
      (:`Remote`
        (`/Engine/EditorBlueprintResources/StandardMacros.FlipFlop`
          (:`A`
            _))))
    (`self.FinishQuestByServer`)))

(event `self.BPDead`
  ;[1 1 1] WeaponManager
  (`/Engine/EditorBlueprintResources/ActorMacros.Switch Has Authority`
    (:`Authority`
      (`self.ReplicatedDeathToAll`))
    (:`Remote`
      (`self.ReplicatedDeathOnServer`))))

(event `ReplicatedDeathOnServer`
  ;[1 1 1] WeaponManager
  (`self.SetDeathStatus` true true :!label _label_6))

(event `ReplicatedDeathToAll`
  ;[1 1 1] WeaponManager
  (goto _label_6))

(event `self.BPShowProgressQuest`
  (`/Game/Widget/InGameWidget.NewCooldownQuest` (`self.WidgetInGame`) (`self.TriggeredDuration`)))

(event `self.BPPower`
  (params (HaveCD :type Boolean) (Delay :type "Float (single-precision)"))
  ;[1 1 1] WeaponManager
  (if HaveCD
    (`/Game/Widget/InGameWidget.LaunchPower1` (`self.WidgetInGame`) Delay)))

(event `FinishQuestByServer`
  (bind _asgame_mode_multi (cast `/Game/Blueprints/Multiplayer/GameModeMulti` (`GameplayStatics.GetGameMode`)))
  (`/Game/Blueprints/Multiplayer/GameModeMulti.CheckQuestVictoryToAll` _asgame_mode_multi))

(event `self.BPPower2`
  (params (HaveCD :type Boolean) (Delay :type "Float (single-precision)"))
  ;[1 1 1] WeaponManager
  (if HaveCD
    (`/Game/Widget/InGameWidget.LaunchPower2` (`self.WidgetInGame`) Delay)))

(event `CheckFinalKill`
  (bind _asgame_mode_multi (cast `/Game/Blueprints/Multiplayer/GameModeMulti` (`GameplayStatics.GetGameMode`)))
  (`/Game/Blueprints/Multiplayer/GameModeMulti.CheckAllDeath` _asgame_mode_multi))

(event `BP CheckKill`
  (`/Engine/EditorBlueprintResources/ActorMacros.Switch Has Authority`
    (:`Authority`
      (`/Engine/EditorBlueprintResources/StandardMacros.FlipFlop`
        (:`A`
          _)))
    (:`Remote`
      (`/Engine/EditorBlueprintResources/StandardMacros.FlipFlop`
        (:`A`
          _))))
  (`self.CheckFinalKill`))

(event `VictoryGoodOnClient`
  (bind _returnvalue (`self.GetRoleParameters`))
  (if (`|EnumEquality` (`.typeOfRoles` (break `InfoRole` _returnvalue)) "Good")
    (`self.IsVictory`)
    (else
      (`self.IsDefeat`))))

(event `VictoryEvilOnClient`
  (bind _returnvalue (`self.GetRoleParameters`))
  (if (`|EnumEquality` (`.typeOfRoles` (break `InfoRole` _returnvalue)) "Naughty")
    (`self.IsVictory`)
    (else
      (`self.IsDefeat`))))

(event `self.OverlapBox.OnComponentBeginOverlap`
  (params (OverlappedComponent :type "PrimitiveComponent Object Reference") (OtherActor :type "Actor Object Reference") (OtherComp :type "PrimitiveComponent Object Reference") (OtherBodyIndex :type Integer) (bFromSweep :type Boolean) (SweepResult :type "HitResult Structure (by ref)"))
  ;[1 1 1] a pas supprimer
)

(fn `DropItem`
  (bind _weaponequipped (`self.WeaponEquipped`))
  (bind _returnvalue (+ (+ (`self.K2_GetActorLocation`) (* (`self.GetActorForwardVector`) (100.0 100.0 0.0))) (0.0 0.0 10.0)))
  (if (!= (`self.WeaponEquipped`) null)
    (bind _outhits (`KismetSystemLibrary.LineTraceMulti` _returnvalue (+ _returnvalue (0.0 0.0 -200.0)) "TraceTypeQuery1"))
    (`self.K2_DetachFromActor` _weaponequipped "KeepWorld" "KeepWorld" "KeepWorld")
    (bind (_output_bblockinghit _output_binitialoverlap _output_time _output_distance _output_location) (`GameplayStatics.BreakHitResult` (`|GetArrayItem` _outhits)))
    (`Weapon.BPDropWeapon` _weaponequipped _output_location)))

(fn `InitCam`)

(fn `InitPower`
  (bind _returnvalue (`self.GetRoleParameters`))
  (`/Game/Widget/InGameWidget.InitPower` (`self.WidgetInGame`) (`self.TESTNAMEPOWER1`) (and (`|EnumEquality` (`.typeOfRoles` (break `InfoRole` _returnvalue)) "Naughty") (`self.HavePower2`)) (`self.TESTNAMEPOWER2`)))

(fn `IsDefeat`
  (bind _widgetingame (`self.WidgetInGame`))
  (`/Game/Widget/InGameWidget.ShowHideInGame` _widgetingame "Hidden")
  (`Widget.SetVisibility` (`/Game/Widget/InGameWidget.DefeatPanel` _widgetingame) "Visible")
  (`/Engine/EditorBlueprintResources/ActorMacros.Switch Has Authority`
    (:`Authority`
      (`Widget.SetVisibility` (`/Game/Widget/InGameWidget.ButtonReturnLobby` _widgetingame) "Visible"))))

(fn `IsVictory`
  (bind _widgetingame (`self.WidgetInGame`))
  (`/Game/Widget/InGameWidget.ShowHideInGame` _widgetingame "Hidden")
  (`Widget.SetVisibility` (`/Game/Widget/InGameWidget.VictoryPanel` _widgetingame) "Visible")
  (`/Engine/EditorBlueprintResources/ActorMacros.Switch Has Authority`
    (:`Authority`
      (`Widget.SetVisibility` (`/Game/Widget/InGameWidget.ButtonReturnLobby` _widgetingame) "Visible"))))

(fn `SetTrap`
  (bind _returnvalue (+ (+ (`self.K2_GetActorLocation`) (* (`self.GetActorForwardVector`) (100.0 100.0 0.0))) (0.0 0.0 10.0)))
  (bind _outhits (`KismetSystemLibrary.LineTraceMulti` :`Start` _returnvalue :`End` (+ _returnvalue (0.0 0.0 -200.0)) :`TraceChannel` "TraceTypeQuery1" :`DrawDebugType` "Persistent"))
  (`self.K2_DetachFromActor` (`self.WeaponEquipped`) "KeepWorld" "KeepWorld" "KeepWorld")
  (bind (_output_bblockinghit _output_binitialoverlap _output_time _output_distance _output_location) (`GameplayStatics.BreakHitResult` (`|GetArrayItem` _outhits)))
  (`self.K2_SetActorTransform` (`self.WeaponEquipped`) (`KismetMathLibrary.MakeTransform` _output_location) false false))

(fn `UserConstructionScript`)