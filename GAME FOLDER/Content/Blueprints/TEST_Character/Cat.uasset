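; Cat character Blueprint, a child class whose power toggles an alternate camera look and lighting.
; BPPower flip-flops between RectLight with full FollowCamera post-process and no post-process, where SpotLight replaces RectLight if GameStateMulti reports night and RectLight is simply hidden otherwise.
; InitCam extends the parent setup by initializing camera post-process with the GoodCat and EvilCat variants.
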(event `self.ReceiveBeginPlay`
  (`parent.ReceiveBeginPlay`))

(event `self.BPPower`
  (bind _followcamera (`self.FollowCamera`))
  (`/Engine/EditorBlueprintResources/StandardMacros.FlipFlop`
    (:`A`
      (`self.SwitchLights` (`self.RectLight`) (`self.SpotLight`))
      (`CameraComponent.SetPostProcessBlendWeight` _followcamera 1.0))
    (:`B`
      (`CameraComponent.SetPostProcessBlendWeight` _followcamera 0.0)
      (bind _asgame_state_multi (cast `/Game/Blueprints/Multiplayer/GameStateMulti` (`GameplayStatics.GetGameState`)))
      (if (`GameStateUtility.Night` _asgame_state_multi)
        (`self.SwitchLights` (`self.SpotLight`) (`self.RectLight`))
        (else
          (`SceneComponent.SetVisibility` (`self.RectLight`) false true))))))

(fn `InitCam`
  (`parent.InitCam`)
  (`self.InitCamPostProcess` (`self.GoodCat`) (`self.EvilCat`)))

(fn `UserConstructionScript`
  (`parent.UserConstructionScript`))