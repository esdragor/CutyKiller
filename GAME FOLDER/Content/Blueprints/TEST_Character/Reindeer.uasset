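; Reindeer is a test character Blueprint with two powers: a timed speed boost and a blink teleport.
; BPPower raises max walk speed, then sets it to a fixed normal value after a delay.
; BPPower2, only for the Naughty role, projects DistanceMaxBlink along the follow camera's forward vector, keeps the actor's height, and teleports there through Test2 without a sweep.
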(event `self.BPPower`
  (set `CharacterMovementComponent.MaxWalkSpeed` 1000.0 (`self.CharacterMovement`))
  (`KismetSystemLibrary.Delay` 5.0)
  (set `CharacterMovementComponent.MaxWalkSpeed` 500.0 (`self.CharacterMovement`)))

(event `self.BPPower2`
  (bind (_returnvalue_x _returnvalue_y _returnvalue_z) (`KismetMathLibrary.BreakVector` (`self.K2_GetActorLocation`)))
  (bind _followcamera (`self.FollowCamera`))
  (bind _distancemaxblink (`self.DistanceMaxBlink`))
  (bind (_returnvalue_x_2 _returnvalue_y_2) (`KismetMathLibrary.BreakVector` (+ (`SceneComponent.K2_GetComponentLocation` _followcamera) (* (`KismetMathLibrary.GetForwardVector` (`SceneComponent.K2_GetComponentRotation` _followcamera)) (`KismetMathLibrary.MakeVector` _distancemaxblink _distancemaxblink)))))
  (bind _returnvalue (`self.GetRoleParameters`))
  (if (`|EnumEquality` (`.typeOfRoles` (break `InfoRole` _returnvalue)) "Naughty")
    (`self.Test2` (`KismetMathLibrary.MakeVector` _returnvalue_x_2 _returnvalue_y_2 _returnvalue_z))))

(event `Test2`
  (params (NewParam :type "Vector Structure"))
  (`self.K2_SetActorLocation` NewParam false true))

(fn `UserConstructionScript`
  (`parent.UserConstructionScript`))