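; Game state Blueprint that runs a day/night cycle by rotating the level's first DirectionalLight.
; From BeginPlay, a Delay and the NightSunCycle event form a 0.1-second loop that adds pitch from Speed and a single frame's delta time.
; Pitch checks against two thresholds around zero set the Night and Day flags and print a French debug message on each change.
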(event `self.ReceiveBeginPlay`
  (bind _outactors (`GameplayStatics.GetAllActorsOfClass` "/Script/Engine.DirectionalLight"))
  (set `self.Light` (`|GetArrayItem` _outactors))
  (`self.K2_AddActorLocalRotation` (`self.Light`) (`KismetMathLibrary.MakeRotator` 0.0 (* (`GameplayStatics.GetWorldDeltaSeconds`) (`self.Speed`))) false false :!label _label)
  (if (and (not (`self.Night`)) (> (.pitch (.rotation (`self.GetTransform` (`self.Light`)))) -0.1))
    (set `self.Night` true)
    (set `self.Day` false)
    (`KismetSystemLibrary.PrintString` "NUIT !!!!!!" true true (struct :`G` 0.66 :`B` 1.0 :`A` 1.0) 10.0)
    (elif (and (not (`self.Day`)) (< (.pitch (.rotation (`self.GetTransform` (`self.Light`)))) 0.1))
      (set `self.Night` false)
      (set `self.Day` true)
      (`KismetSystemLibrary.PrintString` "JOUR !!!!!!" true true (struct :`G` 0.66 :`B` 1.0 :`A` 1.0) 10.0)))
  (`KismetSystemLibrary.Delay` 0.1)
  (`self.NightSunCycle`))

(event `NightSunCycle`
  (goto _label))

(fn `UserConstructionScript`)