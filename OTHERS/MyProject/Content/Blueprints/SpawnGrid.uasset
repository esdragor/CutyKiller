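; SpawnGrid builds a bordered Paper2D tile grid, sized by SizeX and SizeY, when play begins.
; It recreates the tile map with a one-tile margin, draws horizontal and vertical contour tiles around the edge, then fills every interior cell with the Hole tile.
; Vertical walls are written last, so they take the corners.
; BeginPlay ends by printing random integers up to SizeY, which affect no tiles.
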(event `self.ReceiveBeginPlay`
  (`self.ResetTileMap`)
  (`self.SpawnWalls`)
  (`self.SpawnHole`)
  (for _ (range 11)
    (`KismetSystemLibrary.PrintString` (`KismetStringLibrary.Conv_IntToString` (`KismetMathLibrary.RandomIntegerInRange` 1 (`self.SizeY`))))))

(fn `ResetTileMap`
  (`PaperTileMapComponent.CreateNewTileMap` (`PaperTileMapActor.RenderComponent` (`self.TileMap`)) (+ (`self.SizeX`) 2) (+ (`self.SizeY`) 2) 16 16 1.0 true))

(fn `SpawnHole`
  (for _index (range 1 (+ (`self.SizeY`) 1))
    (for _index_2 (range 1 (+ (`self.SizeX`) 1))
      (`PaperTileMapComponent.SetTile` (`PaperTileMapActor.RenderComponent` (`self.TileMap`)) _index_2 _index 0 (`self.Hole`)))))

(fn `SpawnWalls`
  (bind _contourmapvertical (`self.ContourMapVertical`))
  (bind _contourmaphorizontal (`self.ContourMapHorizontal`))
  (bind _rendercomponent (`PaperTileMapActor.RenderComponent` (`self.TileMap`)))
  (for _index (range (+ (+ (`self.SizeX`) 1) 1))
    (`PaperTileMapComponent.SetTile` _rendercomponent _index 0 0 _contourmaphorizontal)
    (`PaperTileMapComponent.SetTile` _rendercomponent _index (+ (`self.SizeY`) 1) 0 _contourmaphorizontal))
  (for _index_2 (range (+ (+ (`self.SizeY`) 1) 1))
    (`PaperTileMapComponent.SetTile` _rendercomponent 0 _index_2 0 _contourmapvertical)
    (`PaperTileMapComponent.SetTile` _rendercomponent (+ (`self.SizeX`) 1) _index_2 0 _contourmapvertical)))

(fn `UserConstructionScript`)